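; Red-team AI drone that flies at living Blue AI and drones and explodes with radial damage when it hits or takes damage.
; Tick picks a target from cached enemies, steers high then descends with direct movement input, and clamps XY to map limits.
; Line traces keep ground clearance and drive a climb-then-forward obstacle bypass.
; Death hides the drone, and ResetToRandomPoint restores it inside its team's spawner box.
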(event Collision|EventHit
  (params (MyComp :type Primitive%20Component%20Object%20Reference) (Other :type Actor%20Object%20Reference) (OtherComp :type Primitive%20Component%20Object%20Reference) (bSelfMoved :type Boolean) (HitLocation :type Vector :default "0, 0, 0") (HitNormal :type Vector :default "0, 0, 0") (NormalImpulse :type Vector :default "0, 0, 0") (Hit :type Hit%20Result%20Structure%20%28by%20ref%29))
  (bind _self self)
  ;[0.15 0.15 0.15 0.5] Drone hits
  (Variables|Default|SetHitsAmount 0)
  (Effects|SpawnEmitteratLocation "/Game/MilitaryWeapDark/FX/P_RocketLauncher_Explosion_01.P_RocketLauncher_Explosion_01" HitLocation "0, 0, 0" "0.400000,0.400000,0.400000")
  (CallFunction|SetDead)
  (CallFunction|CalcEnemyHits HitLocation)
  (Rendering|Debug|DrawDebugSphere HitLocation 2.5e+02 12 "(R=0.000000,G=1.000000,B=0.012230,A=1.000000)" 5.0)
  (Game|Damage|ApplyRadialDamage 2.0 (+ HitLocation "0.000000,0.000000,10.000000") 2.5e+02 0 (Utilities|Array|MakeArray _self) _self 0 true "ECC_GameTraceChannel1"))

(event Collision|EventActorBeginOverlap
  (params (OtherActor :type Actor%20Object%20Reference)))

(event Game|Damage|EventAnyDamage
  (params (Damage :type Float%20%28single-precision%29) (DamageType :type Damage%20Type%20Object%20Reference) (InstigatedBy :type Controller%20Object%20Reference) (DamageCauser :type Actor%20Object%20Reference))
  (bind _returnvalue (Transformation|GetActorLocation))
  (bind _self self)
  ;[0.15 0.15 0.15 0.5] Drone is hit
  (Variables|Default|SetHitsAmount 0)
  (Effects|SpawnEmitteratLocation "/Game/MilitaryWeapDark/FX/P_RocketLauncher_Explosion_01.P_RocketLauncher_Explosion_01" _returnvalue "0, 0, 0" "0.400000,0.400000,0.400000")
  (CallFunction|SetDead)
  (CallFunction|CalcEnemyHits _returnvalue)
  (Rendering|Debug|DrawDebugSphere _returnvalue 2.5e+02 12 "(R=1.000000,G=1.000000,B=1.000000,A=1.000000)" 5.0)
  (Game|Damage|ApplyRadialDamage 2.0 (+ _returnvalue "0.000000,0.000000,10.000000") 2.5e+02 0 (Utilities|Array|MakeArray _self) _self 0 true "ECC_GameTraceChannel1"))

(event EventBeginPlay)

(event EventTick
  (params (DeltaSeconds :type Float%20%28single-precision%29))
  (bind _self self)
  (bind _self_2 self)
  (bind _self_3 self)
  (bind _self_4 self)
  (bind _returnvalue (Transformation|GetActorLocation _self_2))
  (bind _returnvalue_2 (Transformation|GetActorLocation _self_3))
  (bind _returnvalue_3 (Transformation|GetVelocity _self_4))
  (bind _returnvalue_4 (Transformation|GetActorForwardVector _self))
  (bind _returnvalue_5 (Math|Vector|VectorLength _returnvalue_3))
  (Utilities|FlowControl|Sequence
    (:then_0
      (Variables|Default|SetValid%20Nearest%20Enemy%20Received false)
      (bind _enemyseen_temp (CallFunction|MinDistanceSimple))
      (bind _nearestenemy (CallFunction|FindNearestEnemyfromArray _enemyseen_temp))
      (Utilities|IsValid _nearestenemy
        (:Is%20Valid
          (Variables|Default|SetNearestEnemy _nearestenemy)
          (Variables|Default|SetValid%20Nearest%20Enemy%20Received true))
        (:Is%20Not%20Valid
          (Variables|Default|SetValid%20Nearest%20Enemy%20Received false))))
    (:then_1
      (if (Variables|Default|GetValid%20Nearest%20Enemy%20Received)
        (CallFunction|TraceUnder)))
    (:then_2
      (if (Variables|Default|GetValid%20Nearest%20Enemy%20Received)
        (CallFunction|MovetoEnemy)))
    (:then_3
      (if (Variables|Default|GetValid%20Nearest%20Enemy%20Received)
        (if (not (Variables|Default|GetIgnoreObstacle))
          (if (Variables|Default|GetMoving%20Around%20Obstacle%20Up)
            (if (Utilities|Operators|EqualEqual :A (Transformation|GetVelocity self))
              (Variables|Default|SetDroppingVelocity false)
              (Pawn|Input|AddMovementInput (Math|Vector|MakeVector 0.0 0.0 1.0) 0.3 true :!label _label)
              (elif (Variables|Default|GetDroppingVelocity)
                (Pawn|Input|AddMovementInput (Math|Vector|MakeVector 0.0 0.0 0.0) 0.0 true)
                (elif (< (.z (Transformation|GetActorLocation)) (+ (Variables|Default|GetTemp_Height_Obstacle) 1.5e+02))
                  (goto _label)
                  (else
                    (Variables|Default|SetMoving%20Around%20Obstacle%20Up false)
                    (Variables|Default|SetMoving%20Around%20Obstacle%20Forward true)
                    (Components|Movement|StopMovementImmediately (Variables|Character|GetCharacterMovement))
                    (Variables|Default|SetTemp%20Actor%20Position%20For%20Forward%20Obstacle (Transformation|GetActorLocation))
                    (Pawn|Input|AddMovementInput _returnvalue_4 0.2 true)))))
            (elif (Variables|Default|GetMoving%20Around%20Obstacle%20Forward)
              (bind _returnvalue_6 (Transformation|GetActorLocation))
              (if (< (Math|Float|Absolute(Float) (Math|Vector|VectorLength (- _returnvalue_6 (Variables|Default|GetTemp%20Actor%20Position%20For%20Forward%20Obstacle)))) (+ (Variables|Default|GetDistance%20to%20Obstacle) 7.5e+02))
                (Pawn|Input|AddMovementInput _returnvalue_4 0.3 true)
                (else
                  (Variables|Default|SetMoving%20Around%20Obstacle%20Forward false)
                  (Components|Movement|StopMovementImmediately (Variables|Character|GetCharacterMovement))
                  (bind (_outhit _returnvalue_7) (Collision|LineTraceByChannel (Transformation|GetActorLocation self) (Transformation|GetActorLocation (Variables|Default|GetNearestEnemy)) "TraceTypeQuery1" false 0 "None" true "(R=1.000000,G=0.861269,B=0.000000,A=1.000000)"))
                  (if _returnvalue_7
                    (if (Class|GameplayStatics|ObjectIsA (.HitActor (Collision|BreakHitResult _outhit)) "/Game/CharacterAssets/Players/AI/BP_AI_Blue.BP_AI_Blue_C")
                      (Variables|Default|SetIgnoreObstacle true)
                      (else
                        (Variables|Default|SetIgnoreObstacle false)))
                    (else
                      (Variables|Default|SetIgnoreObstacle false)))))
              (else
                (if (> _returnvalue_5 5e+02)
                  (Variables|Default|SetTraceLength (/ _returnvalue_5 1.5))
                  (else
                    (Variables|Default|SetTraceLength (Math|Float|MakeLiteralFloat 3.5e+02))))
                (bind (_outhit_2 _returnvalue_8) (Collision|LineTraceByChannel _returnvalue (+ _returnvalue (* (Transformation|GetActorForwardVector self) (Variables|Default|GetTraceLength))) "TraceTypeQuery1" false 0 "None"))
                (if _returnvalue_8
                  (if (< (.z (Transformation|GetActorLocation)) (+ (.z (.Origin (Collision|GetActorBounds (.HitActor (Collision|BreakHitResult _outhit_2)) false false))) (.z (.BoxExtent (Collision|GetActorBounds (.HitActor (Collision|BreakHitResult _outhit_2)) false false)))))
                    (if (> (+ (.x (.Origin (Collision|GetActorBounds (.HitActor (Collision|BreakHitResult _outhit_2)) false false))) (.x (.BoxExtent (Collision|GetActorBounds (.HitActor (Collision|BreakHitResult _outhit_2)) false false)))) (+ (.y (.Origin (Collision|GetActorBounds (.HitActor (Collision|BreakHitResult _outhit_2)) false false))) (.y (.BoxExtent (Collision|GetActorBounds (.HitActor (Collision|BreakHitResult _outhit_2)) false false)))))
                      (Variables|Default|SetTemp_Width_Obstacle (+ (.x (.Origin (Collision|GetActorBounds (.HitActor (Collision|BreakHitResult _outhit_2)) false false))) (.x (.BoxExtent (Collision|GetActorBounds (.HitActor (Collision|BreakHitResult _outhit_2)) false false)))))
                      (else
                        (Variables|Default|SetTemp_Width_Obstacle (+ (.y (.Origin (Collision|GetActorBounds (.HitActor (Collision|BreakHitResult _outhit_2)) false false))) (.y (.BoxExtent (Collision|GetActorBounds (.HitActor (Collision|BreakHitResult _outhit_2)) false false)))))))
                    (if (not (Variables|Default|GetMoving%20Around%20Obstacle%20Up))
                      (Variables|Default|SetTemp_Height_Obstacle (+ (.Z (Math|Vector|BreakVector (.ImpactPoint (Collision|BreakHitResult _outhit_2)))) 2e+02))
                      (Pawn|Input|AddMovementInput (Math|Vector|MakeVector -1.0 -1.0 -1.0) 1.0 true)
                      (if (Utilities|Operators|EqualEqual :A (Transformation|GetVelocity self))
                        (Pawn|Input|AddMovementInput (Math|Vector|MakeVector 0.0 0.0 1.0) 0.3 true)
                        (Variables|Default|SetDistance%20to%20Obstacle (Math|Float|Absolute(Float) (Math|Vector|VectorLength (- (Transformation|GetActorLocation self) (.ImpactPoint (Collision|BreakHitResult _outhit_2))))))
                        (else
                          (Variables|Default|SetDroppingVelocity true)))
                      (Variables|Default|SetMoving%20Around%20Obstacle%20Up true))))))))))
    (:then_4
      (bind (_x_clamped _y_clamped) (CallFunction|MapLimitClamp (.x _returnvalue_2) (.y _returnvalue_2)))
      (Transformation|SetActorLocation (Math|Vector|MakeVector _x_clamped _y_clamped (.z _returnvalue_2)) true false))))

(fn ConstructionScript)

(fn SetDead
  (bind _returnvalue (AI|GetBlackboard 0))
  (Variables|Default|SetIsDead true)
  (Rendering|SetVisibility (Variables|Default|GetDrone) false false)
  (Pawn|Components|CharacterMovement|DisableMovement (Variables|Character|GetCharacterMovement))
  (Input|DisableInput 0)
  (Collision|SetCollisionEnabled (Variables|Collision|GetCapsuleComponent) "NoCollision")
  (Collision|SetCollisionEnabled (Variables|Default|GetDrone) "NoCollision")
  (Collision|SetCollisionEnabled (Variables|Character|GetMesh) "NoCollision")
  (AI|Components|Blackboard|SetValueasBool _returnvalue (Utilities|String|StringToName (Utilities|String|MakeLiteralString "IsMoving")) false)
  (AI|Components|Blackboard|SetValueasBool _returnvalue (Utilities|String|StringToName (Utilities|String|MakeLiteralString "IsDead")) true))

(fn ResettoRandomPoint
  (bind _returnvalue (AI|GetBlackboard 0))
  (Variables|Default|SetIsDead false)
  (Variables|Default|SetDeadWasCounted false)
  (Rendering|SetVisibility (Variables|Default|GetDrone) true false)
  (Pawn|Components|CharacterMovement|SetMovementMode (Variables|Character|GetCharacterMovement) "MOVE_Flying" 0)
  (Input|EnableInput 0)
  (Transformation|SetRelativeTransform (Variables|Character|GetMesh) (Math|Transform|MakeTransform "0.000000,0.000000,-89.000000" "0.000000,270.000000,0.000000" "1.000000,1.000000,1.000000") false false)
  (if (Actor|ActorHasTag self "Blue")
    (bind _returnvalue_2 (Actor|GetActorOfClass "/Game/CharacterAssets/Players/Spawner/BP_Spawner_Drones_Blue.BP_Spawner_Drones_Blue_C"))
    (Transformation|SetActorTransform (Math|Transform|MakeTransform (Math|Random|RandomPointinBoundingBox (Variables|/Script/Engine.SceneComponent|GetRelativeLocation (Variables|/Game/CharacterAssets/Players/Spawner/BP_Spawner_Drones_Blue.BP_Spawner_Drones_Blue_C|GetBox _returnvalue_2)) (Components|Box|GetScaledBoxExtent (Variables|/Game/CharacterAssets/Players/Spawner/BP_Spawner_Drones_Blue.BP_Spawner_Drones_Blue_C|GetBox _returnvalue_2))) (Math|Rotator|MakeRotator 0.0 0.0 (Math|Random|RandomFloatinRange 0.0 3.6e+02)) "1.000000,1.000000,1.000000") false true)
    (else
      (bind _returnvalue_3 (Actor|GetActorOfClass "/Game/CharacterAssets/Players/Spawner/BP_Spawner_Drones_Red.BP_Spawner_Drones_Red_C"))
      (Transformation|SetActorTransform (Math|Transform|MakeTransform (Math|Random|RandomPointinBoundingBox (Variables|/Script/Engine.SceneComponent|GetRelativeLocation (Variables|/Game/CharacterAssets/Players/Spawner/BP_Spawner_Drones_Red.BP_Spawner_Drones_Red_C|GetBox _returnvalue_3)) (Components|Box|GetScaledBoxExtent (Variables|/Game/CharacterAssets/Players/Spawner/BP_Spawner_Drones_Red.BP_Spawner_Drones_Red_C|GetBox _returnvalue_3))) (Math|Rotator|MakeRotator 0.0 0.0 (Math|Random|RandomFloatinRange 0.0 3.6e+02)) "1.000000,1.000000,1.000000") false true)))
  (Collision|SetCollisionEnabled (Variables|Collision|GetCapsuleComponent) "QueryAndProbe")
  (Collision|SetCollisionEnabled (Variables|Default|GetDrone) "QueryAndProbe")
  (Collision|SetCollisionEnabled (Variables|Character|GetMesh) "QueryAndProbe")
  (AI|Components|Blackboard|SetValueasBool _returnvalue (Utilities|String|StringToName (Utilities|String|MakeLiteralString "IsMoving")) false)
  (AI|Components|Blackboard|SetValueasBool _returnvalue (Utilities|String|StringToName (Utilities|String|MakeLiteralString "IsDead")) false)
  (Variables|Default|SetStart%20Location (Transformation|GetActorLocation))
  (Variables|Default|SetIsMoving false)
  (Variables|Default|SetTimerSet false)
  (Variables|Default|SetinProcessOfmovement false)
  (Variables|Default|SetMoving%20Around%20Obstacle%20Up false)
  (Variables|Default|SetDroppingVelocity false)
  (Variables|Default|SetMoving%20Around%20Obstacle%20Forward false)
  (Variables|Default|SetIgnoreObstacle false)
  (Variables|Default|SetValid%20Nearest%20Enemy%20Received false)
  (Variables|Default|SetDropped%20Velocity%20over%20enemy false))

(fn CalcEnemyHits
  (params (Explosion%20Location :type Vector))
  (bind _outactors (Collision|SphereOverlapActors Explosion%20Location 2.5e+02 (Variables|Default|GetTempEnum) "/Game/CharacterAssets/Players/AI/BP_AI_Blue.BP_AI_Blue_C"))
  (for _array_element _outactors
    (Variables|Default|SetHitsAmount (+ (Variables|Default|GetHitsAmount) 1))))

(fn SetIsMoving
  (Variables|Default|SetIsMoving false)
  (Variables|Default|SetTimerSet false))

(fn FindNearestEnemyfromArray
  (params (SeenEnemies :type Array%20of%20Actor%20Object%20References))
  (if (Utilities|Array|IsNotEmpty SeenEnemies)
    (Variables|Default|SetminDistance 0.0)
    (Variables|Default|SetinProcessOfmovement true)
    (for (_array_element _array_index) SeenEnemies
      (bind _asplayer_parent (Utilities|Casting|CastToPlayer_Parent _array_element))
      (if (Variables|/Game/CharacterAssets/Players/Player_Parent.Player_Parent_C|GetIsDead _asplayer_parent)
        (Utilities|Array|RemoveIndex SeenEnemies _array_index)
        (elif (< (Math|Vector|Distance(Vector) (Transformation|GetActorLocation self) (Transformation|GetActorLocation _array_element)) (Variables|Default|GetminDistance))
          (Variables|Default|SetminDistance (Math|Vector|Distance(Vector) (Transformation|GetActorLocation self) (Transformation|GetActorLocation _array_element)))
          (Variables|Default|SetArrayIndex _array_index))))
    (return (Utilities|Array|Get(acopy) SeenEnemies (Variables|Default|GetArrayIndex)))))

(fn MinDistanceSimple
  (bind _enemyseen_temp (Variables|Default|GetEnemyseen_temp))
  (bind _knownenemies (Variables|Default|GetKnownEnemies))
  (Development|PrintString "started")
  (if (Utilities|Array|IsNotEmpty _knownenemies)
    _
    (else
      (bind _outactors (Actor|GetAllActorswithTag "Blue"))
      (for _array_element _outactors
        (bind _asplayer_parent (Utilities|Casting|CastToPlayer_Parent _array_element))
        (Utilities|Array|Add (Variables|Default|GetKnownEnemies) _asplayer_parent))
      (if (Utilities|Array|IsNotEmpty (Variables|Default|GetKnownEnemies))
        _
        (else
          (return 0.0 0)))))
  (Utilities|Array|Clear _enemyseen_temp)
  (for _array_element_2 _knownenemies
    (bind _asplayer_parent_2 (Utilities|Casting|CastToPlayer_Parent _array_element_2))
    (if (not (Variables|/Game/CharacterAssets/Players/Player_Parent.Player_Parent_C|GetIsDead _asplayer_parent_2))
      (if (Class|GameplayStatics|ObjectIsA _array_element_2 "/Game/CharacterAssets/Players/AI/BP_AI_Blue.BP_AI_Blue_C")
        (Utilities|Array|Add _enemyseen_temp _array_element_2 :!label _label)
        (elif (Class|GameplayStatics|ObjectIsA _array_element_2 "/Game/CharacterAssets/Players/AI/Drone/BP_AI_Drone_BLUE_Final.BP_AI_Drone_BLUE_Final_C")
          (goto _label)))))
  (return 0.0 (Variables|Default|GetEnemyseen_temp)))

(fn SetIsMovingAroundObstacle
  (Variables|Default|SetMoving%20Around%20Obstacle%20Up false))

(fn TraceUnder
  (bind _self self)
  (bind _returnvalue (Transformation|GetActorLocation _self))
  (if (>= (Math|Float|Absolute(Float) (Math|Vector|VectorLength (- (Transformation|GetActorLocation self) (Transformation|GetActorLocation (Variables|Default|GetNearestEnemy))))) 1.5e+03)
    (bind (_outhit _returnvalue_2) (Collision|LineTraceByChannel _returnvalue (+ _returnvalue (* (Transformation|GetActorUpVector self) -4.5e+02)) "TraceTypeQuery3" false 0 "None" true "(R=1.000000,G=0.000000,B=0.821446,A=1.000000)"))
    (if _returnvalue_2
      (if (Utilities|Enum|Equal(Enum) (Collision|GetCollisionObjectType (.HitComponent (Collision|BreakHitResult _outhit))) "ECC_WorldStatic")
        (Pawn|Input|AddMovementInput (Math|Vector|MakeVector 0.0 0.0 1.0) 0.3 true)))))

(fn MovetoEnemy
  (bind _self self)
  (bind _nearestenemy (Variables|Default|GetNearestEnemy))
  (bind _nearestenemy_2 (Variables|Default|GetNearestEnemy))
  (bind _returnvalue (Transformation|GetActorLocation _nearestenemy))
  (bind _returnvalue_2 (Transformation|GetActorLocation _self))
  (bind _returnvalue_3 (Transformation|GetActorLocation _nearestenemy_2))
  (if (not (or (Variables|Default|GetMoving%20Around%20Obstacle%20Up) (Variables|Default|GetMoving%20Around%20Obstacle%20Forward)))
    (if (Math|Boolean|ANDBoolean (<= (Math|Float|Absolute(Float) (- (.z _returnvalue_2) (.z _returnvalue))) 5.3e+03) (<= (Math|Float|Absolute(Float) (- (.x _returnvalue_2) (.x _returnvalue))) 1e+03) (<= (Math|Float|Absolute(Float) (- (.y _returnvalue_2) (.y _returnvalue))) 1e+03))
      (Variables|Default|SetTemp%20Move%20Target%20Height 0.0 :!label _label)
      (Variables|Default|SetTemp%20Random%20Float 0.0)
      (Variables|Default|SetTemp_Scale_Value 0.25)
      (Variables|Default|SetTemp_Scale_Value_XY 1.2)
      (if (Variables|Default|GetDropped%20Velocity%20over%20enemy)
        (bind (_x_clamped _y_clamped) (CallFunction|MapLimitClamp (+ (.x _returnvalue_3) (Math|Random|RandomFloatinRange (* (Variables|Default|GetTemp%20Random%20Float) -1.0) (Variables|Default|GetTemp%20Random%20Float))) (+ (.y _returnvalue_3) (Math|Random|RandomFloatinRange (* (Variables|Default|GetTemp%20Random%20Float) -1.0) (Variables|Default|GetTemp%20Random%20Float))) :!label _label_2))
        (bind _output_get (Variables|Default|SetTempLocation (Math|Rotator|GetRotationXVector (Math|Rotator|FindLookatRotation (Transformation|GetActorLocation self) (Math|Vector|MakeVector _x_clamped _y_clamped (+ (+ (.z _returnvalue_3) (Variables|Default|GetTemp%20Move%20Target%20Height)) (Math|Random|RandomFloatinRange (* (Variables|Default|GetTemp%20Random%20Float) -1.0) (Variables|Default|GetTemp%20Random%20Float))))))))
        (Pawn|Input|AddMovementInput self (Math|Vector|MakeVector 0.0 0.0 (.z _output_get)) (Variables|Default|GetTemp_Scale_Value) true)
        (Pawn|Input|AddMovementInput self (Math|Vector|MakeVector (.x _output_get) (.y _output_get) 0.0) (Variables|Default|GetTemp_Scale_Value_XY) true)
        (Transformation|SetActorRotation (Math|Rotator|Lerp(Rotator) (Transformation|GetActorRotation) (Math|Rotator|MakeRotator 0.0 0.0 (.Yaw (Math|Rotator|BreakRotator (Math|Rotator|FindLookatRotation (Transformation|GetActorLocation self) (Math|Vector|MakeVector _x_clamped _y_clamped (+ (+ (.z _returnvalue_3) (Variables|Default|GetTemp%20Move%20Target%20Height)) (Math|Random|RandomFloatinRange (* (Variables|Default|GetTemp%20Random%20Float) -1.0) (Variables|Default|GetTemp%20Random%20Float)))))))) 0.1 true))
        (elif (Utilities|Operators|EqualEqual :A (Transformation|GetVelocity self))
          (Variables|Default|SetDropped%20Velocity%20over%20enemy true)
          (goto _label_2)
          (else
            (Variables|Default|SetDropped%20Velocity%20over%20enemy false))))
      (elif (>= (Math|Float|Absolute(Float) (Math|Vector|VectorLength (- (Transformation|GetActorLocation self) (Transformation|GetActorLocation (Variables|Default|GetNearestEnemy))))) 3.5e+03)
        (Variables|Default|SetTemp%20Move%20Target%20Height 3e+03)
        (Variables|Default|SetTemp%20Random%20Float 0.0)
        (Variables|Default|SetTemp_Scale_Value 1.0)
        (Variables|Default|SetTemp_Scale_Value_XY 1.0)
        (goto _label_2)
        (else
          (goto _label))))))

(fn MapLimitClamp
  (params (X_coord :type Float%20%28double-precision%29) (Y_coord :type Float%20%28double-precision%29))
  (return (Math|Float|Clamp(Float) X_coord -4.65e+03 1.5e+04) (Math|Float|Clamp(Float) Y_coord -1.485e+04 4.77e+03)))

(fn FindRandomLocation
  (bind _returnvalue (Transformation|GetActorLocation))
  (bind _start_location (Variables|Default|GetStart%20Location))
  (Development|PrintString "FindRandomLoc called")
  (Variables|Default|SetInt 0)
  (Variables|Default|SetTargetLocation (Math|Vector|MakeVector (+ (.x _returnvalue) (Math|Random|RandomFloatinRange -1e+03 1e+03)) (+ (.y _returnvalue) (Math|Random|RandomFloatinRange -1e+03 1e+03)) (.z _returnvalue)) :!label _label)
  (if (> (Math|Float|Absolute(Float) (Math|Vector|VectorLength (- (Variables|Default|GetStart%20Location) (Variables|Default|GetTargetLocation)))) (Variables|Default|GetCanRoamRadius))
    (bind _output_get (Variables|Default|SetInt (+ (Variables|Default|GetInt) 1)))
    (if (< _output_get 10)
      (goto _label)
      (else
        (Development|PrintString "FindRandomLoc out. StartLocation:")
        (Development|PrintString (Utilities|String|ToString(Vector) _start_location))
        (return _start_location)))
    (else
      (Development|PrintString "FindRandomLoc out. TargetLocation:")
      (Development|PrintString (Utilities|String|ToString(Vector) (Variables|Default|GetTargetLocation)))
      (return (Variables|Default|GetTargetLocation)))))

(fn MoveAItoLocation
  (params (MoveToLocation :type Vector :default "0, 0, 0") (Threshold :type Float%20%28double-precision%29))
  (bind _returnvalue (Transformation|GetActorLocation))
  (bind (_x _y) (Math|Vector|BreakVector MoveToLocation))
  (bind _returnvalue_2 (Transformation|GetActorLocation))
  (bind _returnvalue_3 (Math|Vector|MakeVector _x _y (.z _returnvalue)))
  (bind _returnvalue_4 (Math|Rotator|FindLookatRotation _returnvalue_2 _returnvalue_3))
  (bind _returnvalue_5 (Math|Rotator|GetRotationXVector (Math|Rotator|MakeRotator 0.0 0.0 (.yaw _returnvalue_4))))
  (Development|PrintString "Move to location called")
  (if (> (Math|Vector|VectorLength (- (Transformation|GetActorLocation) MoveToLocation)) Threshold)
    (Pawn|Input|AddMovementInput _returnvalue_5 1.0 true)
    (Transformation|SetActorRotation (Math|Rotator|Lerp(Rotator) (Transformation|GetActorRotation) (Math|Rotator|MakeRotator 0.0 0.0 (.yaw _returnvalue_4)) 0.1 true))
    (Development|PrintString "Move not complete")
    (return false _returnvalue_5)
    (else
      (Development|PrintString "Move complete")
      (return true "0, 0, 0"))))