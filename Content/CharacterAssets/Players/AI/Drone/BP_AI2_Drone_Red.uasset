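; Red AI drone that sets up its Drone blackboard on its controller, registers itself there and records its spawn location at BeginPlay.
; FindRandomLocation picks a nearby point at the same height within CanRoamRadius of spawn, falling back to spawn after ten failed tries.
; MoveAIToLocation steers by movement input and smoothed yaw instead of navigation, returning true on arrival.
; Both functions print debug strings, and the move call in BeginPlay is disabled.
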(event EventBeginPlay
  (Utilities|FlowControl|Sequence
    (:then_0
      (bind _asbp_ai_controller_drone (Utilities|Casting|CastToBP_AI_Controller_Drone (Pawn|GetController)))
      (bind _output_get (Variables|Default|SetDroneControllerRef _asbp_ai_controller_drone))
      (bind _blackboardcomponent (Class|AIController|UseBlackboard _output_get "/Game/CharacterAssets/Players/AI/Drone/BlackBoard_Drone.BlackBoard_Drone"))
      (bind _output_get_2 (Variables|Default|SetBlackboard%20Component%20Ref _blackboardcomponent))
      (AI|Components|Blackboard|SetValueasObject _output_get_2 (Utilities|Name|MakeLiteralName "Drone") self))
    (:then_1
      (Variables|Default|SetStart%20Location (Transformation|GetActorLocation)))
    (:then_2
      (bind _target (CallFunction|FindRandomLocation))
      (Class|DroneInterface|MoveAItoLocation(Message) self _target 1e+02))))

(event Collision|EventActorBeginOverlap
  (params (OtherActor :type Actor%20Object%20Reference)))

(event EventTick
  (params (DeltaSeconds :type Float%20%28single-precision%29)))

(fn ConstructionScript
  (|CallParentFunction))

(fn FindRandomLocation
  (bind _returnvalue (Transformation|GetActorLocation))
  (bind _start_location (Variables|Default|GetStart%20Location))
  (Development|PrintString "FindRandomLoc called")
  (Variables|Default|SetInt 0)
  (Variables|Default|SetTargetLocation (Math|Vector|MakeVector (+ (.x _returnvalue) (Math|Random|RandomFloatinRange -1e+03 1e+03)) (+ (.y _returnvalue) (Math|Random|RandomFloatinRange -1e+03 1e+03)) (.z _returnvalue)) :!label _label)
  (if (> (Math|Float|Absolute(Float) (Math|Vector|VectorLength (- (Variables|Default|GetStart%20Location) (Variables|Default|GetTargetLocation)))) (Variables|Default|GetCanRoamRadius))
    (bind _output_get (Variables|Default|SetInt (+ (Variables|Default|GetInt) 1)))
    (if (< _output_get 10)
      (goto _label)
      (else
        (Development|PrintString "FindRandomLoc out. StartLocation:")
        (Development|PrintString (Utilities|String|ToString(Vector) _start_location))
        (return _start_location)))
    (else
      (Development|PrintString "FindRandomLoc out. TargetLocation:")
      (Development|PrintString (Utilities|String|ToString(Vector) (Variables|Default|GetTargetLocation)))
      (return (Variables|Default|GetTargetLocation)))))

(fn MoveAItoLocation
  (params (MoveToLocation :type Vector :default "0, 0, 0") (Threshold :type Float%20%28double-precision%29))
  (bind _returnvalue (Transformation|GetActorLocation))
  (bind (_x _y) (Math|Vector|BreakVector MoveToLocation))
  (bind _returnvalue_2 (Transformation|GetActorLocation))
  (bind _returnvalue_3 (Math|Vector|MakeVector _x _y (.z _returnvalue)))
  (bind _returnvalue_4 (Math|Rotator|FindLookatRotation _returnvalue_2 _returnvalue_3))
  (Development|PrintString "Move to location called")
  (if (> (Math|Vector|VectorLength (- (Transformation|GetActorLocation) MoveToLocation)) Threshold)
    (Pawn|Input|AddMovementInput (Math|Rotator|GetRotationXVector (Math|Rotator|MakeRotator 0.0 0.0 (.yaw _returnvalue_4))) 1.0 false)
    (Transformation|SetActorRotation (Math|Rotator|Lerp(Rotator) (Transformation|GetActorRotation) (Math|Rotator|MakeRotator 0.0 0.0 (.yaw _returnvalue_4)) 0.1 true))
    (Development|PrintString "Move not complete")
    (return false)
    (else
      (Development|PrintString "Move complete")
      (return true))))