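; Red-team AI soldier that uses sight perception to turn toward and shoot Blue-team enemies.
; MinDistanceSimple filters perceived actors to living Blue AI and drones, and RotateTowardsEnemy interpolates toward one, meant to be the closest to its facing angle.
; Tick drives turning and firing: a camera-boom trace checks the Blue tag before applying damage, with ammo counting, shot delays and timed reloads.
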(event OnPerceptionUpdated(AIPerception)
  (params (UpdatedActors :type Array%20of%20Actor%20Object%20References))
  (bind _enemyseen_temp (CallFunction|MinDistanceSimple))
  (Variables|Default|SetEnemyseen_temp _enemyseen_temp))

(event EventBeginPlay
  (Utilities|FlowControl|Sequence))

(event EventTick
  (params (DeltaSeconds :type Float%20%28single-precision%29))
  (bind _returnvalue (Transformation|GetActorRotation))
  (bind _temprotator (Variables|Default|GetTempRotator))
  (bind _rotation_action (Variables|Default|GetRotation%20Action))
  (bind _returnvalue_2 (+ (.yaw _returnvalue) _rotation_action))
  (Utilities|FlowControl|Sequence
    (:then_0
      (Transformation|SetActorRotation (Math|Rotator|MakeRotator (.roll _returnvalue) (.pitch _returnvalue) _returnvalue_2))
      (Transformation|SetWorldRotation (Variables|Default|GetFollowCamera) (Math|Rotator|MakeRotator (.roll _returnvalue) (Variables|Default|GetpitchValue) _returnvalue_2) false false))
    (:then_1
      (if (> (Variables|Default|GetAmmo_amount) 0) :!label _label
        (Utilities|FlowControl|DoOnce false :!label _label_2
          (:Completed
            (bind _hitblue (CallFunction|AIShoot))
            (if _hitblue
              (Development|PrintString "Made 1 shot." false false)
              (CallFunction|AmmoCounter)
              (Utilities|FlowControl|Delay 0.3)
              (Utilities|FlowControl|Sequence
                (:then_0
                  (goto _label_2 Reset))
                (:then_1
                  (goto _label)))
              (else
                (goto _label_2 Reset)))))
        (elif (> (Variables|Default|GetMags_amount) 0)
          (Development|PrintString "RELOADING")
          (Utilities|FlowControl|Delay 3.0)
          (CallFunction|MagsCounter))))
    (:then_2
      (if (Variables|Default|GetinProcessOfRotation)
        (if (Utilities|Operators|EqualEqual (Transformation|GetActorRotation) _temprotator 0.01)
          (Variables|Default|SetinProcessOfRotation false)
          (else
            (Transformation|SetActorRotation self _temprotator)))
        (else
          (bind _enemyseen_temp (CallFunction|MinDistanceSimple))
          (Variables|Default|SetEnemyseen_temp _enemyseen_temp)
          (CallFunction|RotateTowardsEnemy (Variables|Default|GetEnemyseen_temp)))))))

(event Collision|EventActorBeginOverlap
  (params (OtherActor :type Actor%20Object%20Reference)))

(fn ConstructionScript
  (|CallParentFunction))

(fn AIShoot
  (bind _weapon (Variables|Default|GetWeapon))
  (bind _cameraboom (Variables|Default|GetCameraBoom))
  (bind _returnvalue (Transformation|GetWorldLocation _cameraboom))
  (if (not (Variables|Default|GetIsDead))
    (Variables|Default|SetHitBlueActor false)
    (bind (_outhit _returnvalue_2) (Collision|LineTraceByChannel _returnvalue (+ _returnvalue (* (Math|Vector|GetForwardVector _cameraboom) 3e+04)) "TraceTypeQuery3" false 0 "ForDuration" true "(R=0.145936,G=0.000000,B=1.000000,A=1.000000)" "(R=0.000000,G=1.000000,B=0.000000,A=1.000000)" 0.5))
    (if _returnvalue_2
      (if (Utilities|Array|IsEmpty (Variables|/Script/Engine.Actor|GetTags (.HitActor (Collision|BreakHitResult _outhit))))
        (Variables|Default|SetHitBlueActor false)
        (else
          ;[0.15 0.15 0.15 0.5] Success detection, check if enemy
          (bind _output_get (Variables|Default|SetHitBlueActor (== (Utilities|Array|Get(acopy) (Variables|/Script/Engine.Actor|GetTags (.HitActor (Collision|BreakHitResult _outhit)))) "Blue")))
          (if _output_get
            (Utilities|FlowControl|DoOnce false
              (:Completed
                (Components|Animation|PlayAnimation _weapon "/Game/MilitaryWeapDark/Weapons/Anims/Fire_Rifle_W.Fire_Rifle_W" false)
                (Collision|LineTraceByChannel (.location (Transformation|GetSocketTransform _weapon "MuzzleFlash" "RTS_World")) (.ImpactPoint (Collision|BreakHitResult _outhit)) "TraceTypeQuery3" false 0 "ForDuration")
                (Game|Damage|ApplyDamage (.HitActor (Collision|BreakHitResult _outhit)) 1.0 0 0))))))
      (return (Variables|Default|GetHitBlueActor) (.HitActor (Collision|BreakHitResult _outhit))))))

(fn RotateTowardsEnemy
  (params (SeenEnemies :type Array%20of%20Actor%20Object%20References))
  (bind _self self)
  (if (Utilities|Array|IsNotEmpty SeenEnemies)
    (Variables|Default|SetminAngle 1.8e+02)
    (Variables|Default|SetinProcessOfRotation true)
    (for (_array_element _array_index) SeenEnemies
      (bind _asplayer_parent (Utilities|Casting|CastToPlayer_Parent _array_element))
      (if (Variables|/Game/CharacterAssets/Players/Player_Parent.Player_Parent_C|GetIsDead _asplayer_parent)
        (Utilities|Array|RemoveIndex SeenEnemies _array_index)
        (elif (< (Class|KismetMathLibrary|DegAcos (Math|Vector|DotProduct (Transformation|GetActorForwardVector _self) (Math|Vector|Normalize (- (Transformation|GetActorLocation _array_element) (Transformation|GetActorLocation _self))))) (Variables|Default|GetminAngle))
          (Variables|Default|SetminAngle (Class|KismetMathLibrary|DegAcos (Math|Vector|DotProduct (Transformation|GetActorForwardVector _self) (Math|Vector|Normalize (- (Transformation|GetActorLocation _array_element) (Transformation|GetActorLocation _self))))))
          (Variables|Default|SetArrayIndex _array_index))))
    (Transformation|SetActorRotation self (Math|Interpolation|RInterpTo (Transformation|GetActorRotation) (Math|Rotator|FindLookatRotation (Transformation|GetActorLocation) (Transformation|GetWorldLocation (Variables|/Script/Engine.Actor|GetRootComponent (Utilities|Array|Get(acopy) SeenEnemies (Variables|Default|GetArrayIndex))))) (Utilities|Time|GetWorldDeltaSeconds) 35.0))
    (Variables|Default|SetTempRotator (Math|Interpolation|RInterpTo (Transformation|GetActorRotation) (Math|Rotator|FindLookatRotation (Transformation|GetActorLocation) (Transformation|GetWorldLocation (Variables|/Script/Engine.Actor|GetRootComponent (Utilities|Array|Get(acopy) SeenEnemies (Variables|Default|GetArrayIndex))))) (Utilities|Time|GetWorldDeltaSeconds) 35.0))
    (return 0 0 (Math|Interpolation|RInterpTo (Transformation|GetActorRotation) (Math|Rotator|FindLookatRotation (Transformation|GetActorLocation) (Transformation|GetWorldLocation (Variables|/Script/Engine.Actor|GetRootComponent (Utilities|Array|Get(acopy) SeenEnemies (Variables|Default|GetArrayIndex))))) (Utilities|Time|GetWorldDeltaSeconds) 35.0))))

(fn MinDistanceSimple
  (bind _enemyseen_temp (Variables|Default|GetEnemyseen_temp))
  (bind _aiperception (Variables|Default|GetAIPerception))
  (bind _outactors (Class|AIPerceptionComponent|GetKnownPerceivedActors _aiperception "/Script/AIModule.AISense_Sight"))
  (Development|PrintString "started")
  (Variables|Default|SetError false)
  (if (Utilities|Array|IsNotEmpty _outactors)
    (bind _output_get (Variables|Default|SetTempPerceptedActors _outactors))
    (Utilities|Array|Clear _enemyseen_temp)
    (for _array_element _output_get
      (bind _asplayer_parent (Utilities|Casting|CastToPlayer_Parent _array_element))
      (if (not (Variables|/Game/CharacterAssets/Players/Player_Parent.Player_Parent_C|GetIsDead _asplayer_parent))
        (if (Class|GameplayStatics|ObjectIsA _array_element "/Game/CharacterAssets/Players/AI/BP_AI_Blue.BP_AI_Blue_C")
          (Utilities|Array|Add _enemyseen_temp _array_element :!label _label)
          (elif (Class|GameplayStatics|ObjectIsA _array_element "/Game/CharacterAssets/Players/BP_Drone_Blue.BP_Drone_Blue_C")
            (goto _label)))))
    (return 0.0 (Variables|Default|GetError) (Variables|Default|GetEnemyseen_temp))
    (else
      (bind _output_get_2 (Variables|Default|SetError true))
      (return 0.0 _output_get_2 0))))