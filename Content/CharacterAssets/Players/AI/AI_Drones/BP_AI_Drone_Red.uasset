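; Red-team AI drone that flies under its own controller and registers as an agent with the red drones' Learning Agents manager.
; On BeginPlay it caches Blue-tagged players as known enemies.
; Each tick it filters these to living blue AI and drones and stores the closest as NearestEnemy.
; Movement input comes separately from X/Y/Z values set outside this graph, not from steering toward that enemy.
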(event EventBeginPlay
  (Utilities|FlowControl|Sequence
    (:then_0
      (bind _outactors (Actor|GetAllActorswithTag "Blue"))
      (for _array_element _outactors
        (bind _asplayer_parent (Utilities|Casting|CastToPlayer_Parent _array_element))
        (Utilities|Array|Add (Variables|Default|GetKnownEnemies) _asplayer_parent))
      (Pawn|SpawnDefaultController)
      (Pawn|Components|CharacterMovement|SetMovementMode (Variables|Character|GetCharacterMovement) "MOVE_Flying" 0))
    (:then_1
      (bind _outactors_2 (Actor|GetAllActorswithTag "LearningAgentsManagerDronesRed"))
      (for _array_element_2 _outactors_2
        (Utilities|IsValid (Actor|GetComponentbyClass _array_element_2 "/Script/LearningAgents.LearningAgentsManager")
          (:Is%20Valid
            (Class|LearningAgentsManager|AddAgent (Actor|GetComponentbyClass _array_element_2 "/Script/LearningAgents.LearningAgentsManager") self)
            (Variables|Default|SetFoundManager true))))
      (if (not (Variables|Default|GetFoundManager))
        (Development|PrintString "COULDN`T FIND LEARNING AGENTS Drones red MANAGER.")))
    (:then_2
      (bind _enemyseen_temp (CallFunction|MinDistanceSimple))
      (bind _nearestenemy (CallFunction|MoveTowardsEnemy _enemyseen_temp))
      (Variables|Default|SetNearestEnemy _nearestenemy))))

(event Collision|EventActorBeginOverlap
  (params (OtherActor :type Actor%20Object%20Reference)))

(event EventTick
  (params (DeltaSeconds :type Float%20%28single-precision%29))
  (Utilities|FlowControl|Sequence
    (:then_0
      (bind _enemyseen_temp (CallFunction|MinDistanceSimple))
      (bind _nearestenemy (CallFunction|MoveTowardsEnemy _enemyseen_temp))
      (Variables|Default|SetNearestEnemy _nearestenemy))
    (:then_1
      (Pawn|Input|AddMovementInput (Math|Vector|MakeVector (* (Variables|Default|GetX_Value) 1.0) (* (Variables|Default|GetY_Value) 1.0) (* (Variables|Default|GetZ_Value) 1.0)) 1.0 false))
    (:then_2
      (bind _outactors (Actor|GetAllActorsOfClass "/Game/CharacterAssets/Players/AI/BP_AI_Blue.BP_AI_Blue_C"))
      (Pawn|Input|AddMovementInput self (Math|Rotator|GetRotationXVector (Math|Rotator|FindLookatRotation (Transformation|GetWorldLocation (Variables|Default|GetDrone)) (Transformation|GetActorLocation (Utilities|Array|Get(acopy) _outactors (Math|Random|RandomInteger 7))))) 1.0 false))))

(fn ConstructionScript
  (|CallParentFunction))

(fn MinDistanceSimple
  (bind _knownenemies (Variables|Default|GetKnownEnemies))
  (bind _enemyseen_temp (Variables|Default|GetEnemyseen_temp))
  (Development|PrintString "started")
  (if (Utilities|Array|IsNotEmpty _knownenemies)
    (Utilities|Array|Clear _enemyseen_temp)
    (for _array_element _knownenemies
      (bind _asplayer_parent (Utilities|Casting|CastToPlayer_Parent _array_element))
      (if (not (Variables|/Game/CharacterAssets/Players/Player_Parent.Player_Parent_C|GetIsDead _asplayer_parent))
        (if (Class|GameplayStatics|ObjectIsA _array_element "/Game/CharacterAssets/Players/AI/BP_AI_Blue.BP_AI_Blue_C")
          (Utilities|Array|Add _enemyseen_temp _array_element :!label _label)
          (elif (Class|GameplayStatics|ObjectIsA _array_element "/Game/CharacterAssets/Players/BP_Drone_Blue.BP_Drone_Blue_C")
            (goto _label)))))
    (return 0.0 (Variables|Default|GetEnemyseen_temp))
    (else
      (return 0.0 0))))

(fn MoveTowardsEnemy
  (params (SeenEnemies :type Array%20of%20Actor%20Object%20References))
  (if (Utilities|Array|IsNotEmpty SeenEnemies)
    (Variables|Default|SetminDistance 1e+06)
    (Variables|Default|SetinProcessOfmovement true)
    (for (_array_element _array_index) SeenEnemies
      (bind _asplayer_parent (Utilities|Casting|CastToPlayer_Parent _array_element))
      (if (Variables|/Game/CharacterAssets/Players/Player_Parent.Player_Parent_C|GetIsDead _asplayer_parent)
        (Utilities|Array|RemoveIndex SeenEnemies _array_index)
        (elif (< (Math|Vector|Distance(Vector) (Transformation|GetActorLocation self) (Transformation|GetActorLocation _array_element)) (Variables|Default|GetminDistance))
          (Variables|Default|SetminDistance (Math|Vector|Distance(Vector) (Transformation|GetActorLocation self) (Transformation|GetActorLocation _array_element)))
          (Variables|Default|SetArrayIndex _array_index))))
    (return (Utilities|Array|Get(acopy) SeenEnemies (Variables|Default|GetArrayIndex)))))