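; Spawner that places red AI drones inside its Box volume, using the count stored in the game instance.
; BeginPlay waits a random interval, then loops over that count with a random Delay before each SpawnRed call.
; SpawnRed picks a random point from the Box's relative location and scaled extent, then spawns the drone with its default controller.
; A similar SpawnDrone function for blue drones is never called here.
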(event EventBeginPlay
  (bind _asgi_my_game_instance (Utilities|Casting|CastToGI_My_GameInstance (Game|GetGameInstance))
    (:then
      (Variables|Default|SetAmount (Variables|/Game/CharacterAssets/Maps/GI_My_GameInstance.GI_My_GameInstance_C|GetDrones%20Red%20Amount _asgi_my_game_instance))
      (Utilities|FlowControl|Delay (Math|Random|RandomFloatinRange 3.0 1e+01))
      (if (!= (Variables|Default|GetAmount) 0)
        (for _index (range 0 (- (Variables|Default|GetAmount) 1))
          (Utilities|FlowControl|Delay (Math|Random|RandomFloatinRange 3.0 6.0))
          (CallFunction|SpawnRed))))
    (:CastFailed
      (Development|PrintString "CAST TO GAME INSTANCE FAILED"))))

(event Collision|EventActorBeginOverlap
  (params (OtherActor :type Actor%20Object%20Reference)))

(event EventTick
  (params (DeltaSeconds :type Float%20%28single-precision%29)))

(fn ConstructionScript)

(fn SpawnDrone
  (bind _box (Variables|Default|GetBox))
  (bind _returnvalue (Game|SpawnActorfromClass "/Game/CharacterAssets/Players/AI/AI_Drones/BP_AI_Drone_Blue.BP_AI_Drone_Blue_C" (Math|Transform|MakeTransform (Math|Random|RandomPointinBoundingBox (Variables|/Script/Engine.SceneComponent|GetRelativeLocation _box) (Components|Box|GetScaledBoxExtent _box)) "0, 0, 0" "1.000000,1.000000,1.000000") "AdjustIfPossibleButAlwaysSpawn" "MultiplyWithRoot" 0 0))
  (Pawn|SpawnDefaultController _returnvalue))

(fn SpawnRed
  (bind _box (Variables|Default|GetBox))
  (for _index (range 0 0)
    (bind _returnvalue (Game|SpawnActorfromClass "/Game/CharacterAssets/Players/AI/Drone/BP_AI_Drone_RED_Final.BP_AI_Drone_RED_Final_C" (Math|Transform|MakeTransform (Math|Random|RandomPointinBoundingBox (Variables|/Script/Engine.SceneComponent|GetRelativeLocation _box) (Components|Box|GetScaledBoxExtent _box)) "0, 0, 0" "1.000000,1.000000,1.000000") "AdjustIfPossibleButAlwaysSpawn" "MultiplyWithRoot" 0 0))
    (Pawn|SpawnDefaultController _returnvalue)))