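; Spawner actor that populates the level with red-team AI soldiers (BP_AI_Red) on BeginPlay.
; It reads the soldier count from the game instance, then spawns each at a reachable navigation point near a random point in its Box.
; Each soldier gets mesh and capsule-height adjustments, a random-point reset and a default controller.
; A simpler single-spawn function is uncalled here, and per-map height logic is disabled.
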(event EventBeginPlay
  (bind _asgi_my_game_instance (Utilities|Casting|CastToGI_My_GameInstance (Game|GetGameInstance))
    (:then
      (Variables|Default|SetAmount (Variables|/Game/CharacterAssets/Maps/GI_My_GameInstance.GI_My_GameInstance_C|GetSoldiers%20Red%20Amount _asgi_my_game_instance))
      (CallFunction|SpawnRedSoldiers))
    (:CastFailed
      (Development|PrintString "CAST TO GAME INSTANCE FAILED"))))

(event Collision|EventActorBeginOverlap
  (params (OtherActor :type Actor%20Object%20Reference)))

(event EventTick
  (params (DeltaSeconds :type Float%20%28single-precision%29)))

(fn ConstructionScript)

(fn SpawnSoldier
  (bind _box (Variables|Default|GetBox))
  (Game|SpawnActorfromClass "/Game/CharacterAssets/Players/AI/BP_AI_Red.BP_AI_Red_C" (Math|Transform|MakeTransform (Math|Random|RandomPointinBoundingBox (Variables|/Script/Engine.SceneComponent|GetRelativeLocation _box) (Components|Box|GetScaledBoxExtent _box)) "0, 0, 0" "1.000000,1.000000,1.000000") "AdjustIfPossibleButAlwaysSpawn" "MultiplyWithRoot" 0 0))

(fn SpawnRedSoldiers
  (bind _box (Variables|Default|GetBox))
  (bind _amount (Variables|Default|GetAmount))
  (if (!= _amount 0)
    (for _index (range 0 (- _amount 1))
      (bind _returnvalue (Game|SpawnActorfromClass "/Game/CharacterAssets/Players/AI/BP_AI_Red.BP_AI_Red_C" (Math|Transform|MakeTransform (.RandomLocation (AI|Navigation|GetRandomReachablePointinRadius (Math|Random|RandomPointinBoundingBox (Variables|/Script/Engine.SceneComponent|GetRelativeLocation _box) (Components|Box|GetScaledBoxExtent _box)) 1e+03 0 0)) "0, 0, 0" "1.000000,1.000000,1.000000") "AdjustIfPossibleButAlwaysSpawn" "MultiplyWithRoot" 0 0))
      (Transformation|SetRelativeTransform (Variables|/Script/Engine.Character|GetMesh _returnvalue) (Math|Transform|MakeTransform (Math|Vector|MakeVector 0.0 0.0 -1e+02) "0.000000,270.000000,0.000000" "1.000000,1.000000,1.000000") false false)
      (Transformation|SetActorTransform _returnvalue (Math|Transform|MakeTransform (Math|Vector|MakeVector (.X (Math|Vector|BreakVector (Transformation|GetActorLocation _returnvalue))) (.Y (Math|Vector|BreakVector (Transformation|GetActorLocation _returnvalue))) (+ (Components|Capsule|GetScaledCapsuleHalfHeight (Variables|/Script/Engine.Character|GetCapsuleComponent _returnvalue)) (.Z (Math|Vector|BreakVector (Transformation|GetActorLocation _returnvalue))))) "0.000000,-90.000000,0.000000" "1.000000,1.000000,1.000000"))
      (Default|ResettoRandomPoint _returnvalue)
      (Pawn|SpawnDefaultController _returnvalue))))