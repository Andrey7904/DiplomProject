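; Blue AI soldier character that takes damage, ragdolls on death and respawns at a random spot.
; AnyDamage prints debug values and lowers Health; at zero it disables movement and input and turns on mesh physics.
; After a three-second delay, ResetToRandomPoint stops physics, calls ResetToDefault, re-seats the mesh and teleports the actor within a hardcoded box with random yaw.
; BeginPlay uses the same reset for initial placement.
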(event Game|Damage|EventAnyDamage
  (params (Damage :type Float%20%28single-precision%29) (DamageType :type Damage%20Type%20Object%20Reference) (InstigatedBy :type Controller%20Object%20Reference) (DamageCauser :type Actor%20Object%20Reference))
  (bind _mesh (Variables|Character|GetMesh))
  ;[0.15 0.15 0.15 0.5] Take Damage
  (Development|PrintString "Current helth:" true true "(R=0.000000,G=0.660000,B=1.000000,A=1.000000)" 5.0)
  (Development|PrintString (Utilities|String|ToString(Float) (- (Variables|Default|GetHealth) Damage)) true true "(R=0.000000,G=0.660000,B=1.000000,A=1.000000)" 5.0)
  (Development|PrintString "Damage:" true true "(R=0.000000,G=0.660000,B=1.000000,A=1.000000)" 5.0)
  (Development|PrintString (Utilities|String|ToString(Float) Damage) true true "(R=0.000000,G=0.660000,B=1.000000,A=1.000000)" 5.0)
  (if (> (Variables|Default|GetHealth) 0.0)
    (Variables|Default|SetHealth (- (Variables|Default|GetHealth) Damage))
    (if (<= (Variables|Default|GetHealth) 0.0)
      (Pawn|Components|CharacterMovement|DisableMovement (Variables|Character|GetCharacterMovement))
      (Input|DisableInput 0)
      (Physics|SetSimulatePhysics _mesh true)
      (Class|SkeletalMeshComponent|SetPhysicsBlendWeight _mesh 1.0)
      (Collision|SetCollisionEnabled _mesh "QueryAndPhysics")
      (Utilities|FlowControl|Delay 3.0)
      (CallFunction|ResettoRandomPoint))))

(event Collision|EventActorBeginOverlap
  (params (OtherActor :type Actor%20Object%20Reference)))

(event EventTick
  (params (DeltaSeconds :type Float%20%28single-precision%29)))

(event EventBeginPlay
  (CallFunction|ResettoRandomPoint))

(fn ConstructionScript
  (|CallParentFunction))

(fn ResettoRandomPoint
  (bind _returnvalue (Math|Random|RandomPointinBoundingBox "1500.000000,1750.000000,0.000000" "1300.000000,1550.000000,0.000000"))
  (bind (_x _y _z) (Math|Vector|BreakVector _returnvalue))
  (Physics|SetSimulatePhysics (Variables|Character|GetMesh) false)
  (Input|EnableInput 0)
  (CallFunction|ResettoDefault)
  (Transformation|SetRelativeTransform (Variables|Character|GetMesh) (Math|Transform|MakeTransform "0.000000,0.000000,-89.000000" "0.000000,270.000000,0.000000" "1.000000,1.000000,1.000000") false false)
  (Transformation|SetActorTransform (Math|Transform|MakeTransform (Math|Vector|MakeVector _x _y (+ (Components|Capsule|GetScaledCapsuleHalfHeight (Variables|Default|GetCapsuleComponent)) _z)) (Math|Rotator|MakeRotator 0.0 0.0 (Math|Random|RandomFloatinRange 0.0 3.6e+02)) "1.000000,1.000000,1.000000") false true))