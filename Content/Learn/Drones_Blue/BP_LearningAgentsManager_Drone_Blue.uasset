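; Learning Agents manager actor for blue AI drones that either trains or runs their neural-network policy, selected by RunInference.
; BeginPlay gathers the drones with a tick prerequisite on itself, then builds interactor, policy, critic, environment and shared-memory PPO trainer from Red-named classes and assets.
; Tick runs policy inference or PPO training; in inference mode, BeginPlay also resets drones to random points.
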(event EventBeginPlay
  (bind _shared_memory_settings (Variables|Default|GetShared%20Memory%20Settings))
  (Utilities|FlowControl|Sequence
    (:then_0
      (bind _outactors (Actor|GetAllActorsOfClass "/Game/CharacterAssets/Players/AI/Drone/BP_AI_Drone_BLUE_Final.BP_AI_Drone_BLUE_Final_C"))
      (bind _output_get (Variables|Default|SetAIActors _outactors))
      (Actor|Tick|AddTickPrerequisiteActor _output_get self))
    (:then_1
      (bind _returnvalue (Class|LearningAgentsInteractor|MakeInteractor (Variables|Default|GetLearningAgentsManager) "/Game/Learn/Soldiers_Red/BP_LearningInteractorRed.BP_LearningInteractorRed_C" "InteractorR"))
      (Variables|Default|SetInteractor _returnvalue))
    (:then_2
      (bind _returnvalue_2 (Class|LearningAgentsPolicy|MakePolicy (Variables|Default|GetLearningAgentsManager) (Variables|Default|GetInteractor) "/Script/LearningAgents.LearningAgentsPolicy" "PolicyRed" "/Game/Learn/Soldiers_Red/DA_NeuralNetworkEncoderRed.DA_NeuralNetworkEncoderRed" "/Game/Learn/Soldiers_Red/DA_NeuralNetworkPolicyRed.DA_NeuralNetworkPolicyRed" "/Game/Learn/Soldiers_Red/DA_NeuralNetworkDecoderRed.DA_NeuralNetworkDecoderRed" false false false (Variables|Default|GetPolicy%20Settings) 1234))
      (Variables|Default|SetPolicy _returnvalue_2))
    (:then_3
      (bind _returnvalue_3 (Class|LearningAgentsCritic|MakeCritic (Variables|Default|GetLearningAgentsManager) (Variables|Default|GetInteractor) (Variables|Default|GetPolicy) "/Script/LearningAgents.LearningAgentsCritic" "CriticRed" "/Game/Learn/Soldiers_Red/DA_NeuralNetworkCriticRed.DA_NeuralNetworkCriticRed" false (Variables|Default|GetCritic%20Settings) 1234))
      (Variables|Default|SetCritic _returnvalue_3))
    (:then_4
      (bind _returnvalue_4 (Class|LearningAgentsTrainingEnvironment|MakeTrainingEnvironment (Variables|Default|GetLearningAgentsManager) "/Game/Learn/Soldiers_Red/BP_LearningTrainerRed.BP_LearningTrainerRed_C" "TrainingEnvironmentRed"))
      (Variables|Default|SetTraining%20Env _returnvalue_4))
    (:then_5
      (bind _returnvalue_5 (Class|LearningAgentsCommunicatorLibrary|SpawnSharedMemoryTrainingProcess (Variables|Default|GetTrainer%20Process%20Settings) _shared_memory_settings))
      (bind _returnvalue_6 (Class|LearningAgentsCommunicatorLibrary|MakeSharedMemoryCommunicator _returnvalue_5 _shared_memory_settings))
      (Variables|Default|SetCommunicator _returnvalue_6))
    (:then_6
      (bind _returnvalue_7 (Class|LearningAgentsPPOTrainer|MakePPOTrainer (Variables|Default|GetLearningAgentsManager) (Variables|Default|GetInteractor) (Variables|Default|GetTraining%20Env) (Variables|Default|GetPolicy) (Variables|Default|GetCritic) (Variables|Default|GetCommunicator) "/Script/LearningAgentsTraining.LearningAgentsPPOTrainer" "PPOTrainer" (Variables|Default|GetTrainer%20Settings)))
      (Variables|Default|SetPPOTrainer _returnvalue_7))
    (:then_7
      (if (Variables|Default|GetRunInference)
        (Default|ResettoRandomPoint (Variables|Default|GetAIActors))))))

(event Collision|EventActorBeginOverlap
  (params (OtherActor :type Actor%20Object%20Reference)))

(event EventTick
  (params (DeltaSeconds :type Float%20%28single-precision%29))
  (if (Variables|Default|GetRunInference)
    (Class|LearningAgentsPolicy|RunInference (Variables|Default|GetPolicy) 0.0)
    (else
      (Class|LearningAgentsPPOTrainer|RunTraining (Variables|Default|GetPPOTrainer) (Variables|Default|GetTrainer%20Training%20Settings) (Variables|Default|GetTraining%20Game%20Settings) true true))))

(fn ConstructionScript)