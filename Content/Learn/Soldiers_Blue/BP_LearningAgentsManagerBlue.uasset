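; Learning Agents manager that trains or runs the neural policy for Blue soldier AI.
; BeginPlay makes itself their tick prerequisite, then builds interactor, policy, critic, environment and shared-memory PPO trainer from Blue network assets without reinitializing them.
; RunInference switches Tick between inference and PPO training, and randomizes agent positions at start when true.
; A function averaging Red agents' hit counts exists, but its timer is unconnected.
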(event EventBeginPlay
  (bind _shared_memory_settings (Variables|Default|GetShared%20Memory%20Settings))
  (Utilities|FlowControl|Sequence
    (:then_0
      (bind _outactors (Actor|GetAllActorsOfClass "/Game/CharacterAssets/Players/AI/BP_AI_Blue.BP_AI_Blue_C"))
      (bind _output_get (Variables|Default|SetAIActors _outactors))
      (Actor|Tick|AddTickPrerequisiteActor _output_get self))
    (:then_1
      (bind _returnvalue (Class|LearningAgentsInteractor|MakeInteractor (Variables|Default|GetLearningAgentsManager) "/Game/Learn/Soldiers_Blue/BP_LearningInteractorBlue.BP_LearningInteractorBlue_C" "InteractorBlue"))
      (Variables|Default|SetInteractor _returnvalue))
    (:then_2
      (bind _returnvalue_2 (Class|LearningAgentsPolicy|MakePolicy (Variables|Default|GetLearningAgentsManager) (Variables|Default|GetInteractor) "/Script/LearningAgents.LearningAgentsPolicy" "PolicyBlue" "/Game/Learn/Soldiers_Blue/DA_NeuralNetworkEncoderBlue.DA_NeuralNetworkEncoderBlue" "/Game/Learn/Soldiers_Blue/DA_NeuralNetworkPolicyBlue.DA_NeuralNetworkPolicyBlue" "/Game/Learn/Soldiers_Blue/DA_NeuralNetworkDecoderBlue.DA_NeuralNetworkDecoderBlue" false false false (Variables|Default|GetPolicy%20Settings) 1234))
      (Variables|Default|SetPolicy _returnvalue_2))
    (:then_3
      (bind _returnvalue_3 (Class|LearningAgentsCritic|MakeCritic (Variables|Default|GetLearningAgentsManager) (Variables|Default|GetInteractor) (Variables|Default|GetPolicy) "/Script/LearningAgents.LearningAgentsCritic" "CriticBlue" "/Game/Learn/Soldiers_Blue/DA_NeuralNetworkCriticBlue.DA_NeuralNetworkCriticBlue" false (Variables|Default|GetCritic%20Settings) 1234))
      (Variables|Default|SetCritic _returnvalue_3))
    (:then_4
      (bind _returnvalue_4 (Class|LearningAgentsTrainingEnvironment|MakeTrainingEnvironment (Variables|Default|GetLearningAgentsManager) "/Game/Learn/Soldiers_Blue/BP_LearningTrainerBlue.BP_LearningTrainerBlue_C" "TrainingEnvironmentBlue"))
      (Variables|Default|SetTraining%20Env _returnvalue_4))
    (:then_5
      (bind _returnvalue_5 (Class|LearningAgentsCommunicatorLibrary|SpawnSharedMemoryTrainingProcess (Variables|Default|GetTrainer%20Process%20Settings) _shared_memory_settings))
      (bind _returnvalue_6 (Class|LearningAgentsCommunicatorLibrary|MakeSharedMemoryCommunicator _returnvalue_5 _shared_memory_settings))
      (Variables|Default|SetCommunicator _returnvalue_6))
    (:then_6
      (bind _returnvalue_7 (Class|LearningAgentsPPOTrainer|MakePPOTrainer (Variables|Default|GetLearningAgentsManager) (Variables|Default|GetInteractor) (Variables|Default|GetTraining%20Env) (Variables|Default|GetPolicy) (Variables|Default|GetCritic) (Variables|Default|GetCommunicator) "/Script/LearningAgentsTraining.LearningAgentsPPOTrainer" "PPOTrainerBlue" (Variables|Default|GetTrainer%20Settings)))
      (Variables|Default|SetPPOTrainer _returnvalue_7))
    (:then_7
      (if (Variables|Default|GetRunInference)
        (Default|ResettoRandomPoint (Variables|Default|GetAIActors))))))

(event Collision|EventActorBeginOverlap
  (params (OtherActor :type Actor%20Object%20Reference)))

(event EventTick
  (params (DeltaSeconds :type Float%20%28single-precision%29))
  (if (Variables|Default|GetRunInference)
    (Class|LearningAgentsPolicy|RunInference (Variables|Default|GetPolicy) 0.0)
    (else
      (Class|LearningAgentsPPOTrainer|RunTraining (Variables|Default|GetPPOTrainer) (Variables|Default|GetTrainer%20Training%20Settings) (Variables|Default|GetTraining%20Game%20Settings) true true))))

(fn ConstructionScript)

(fn CalcAgentEfficiency
  (bind _outactors (Actor|GetAllActorsOfClass "/Game/CharacterAssets/Players/AI/BP_AI_Red.BP_AI_Red_C"))
  (for _array_element _outactors
    (Utilities|Array|Add (Variables|Default|GetHits%20Amount%20Array) (Variables|/Game/CharacterAssets/Players/AI/BP_AI_Parent.BP_AI_Parent_C|GetAmountOfHits _array_element))
    (Variables|Default|SethitsSum (+ (Variables|Default|GethitsSum) (Variables|/Game/CharacterAssets/Players/AI/BP_AI_Parent.BP_AI_Parent_C|GetAmountOfHits _array_element))))
  (Variables|Default|SetAvgHitsAmount (/ (Variables|Default|GethitsSum) (Utilities|Array|Length (Variables|Default|GetHits%20Amount%20Array)))))