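; Learning Agents trainer for the blue AI soldiers (BP_AI_Blue), defining their rewards, completions and episode resets.
; Reward combines a bonus for hitting red, a small death penalty and a rank-scaled term, though WasRanked is cleared before that term is read.
; Completion consumes each agent's termination flag, and reset moves the agent to a random point.
; A periodic check to terminate agents without recent hits exists, but its call is disabled.
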(fn GatherAgentReward
  (params (AgentId :type Integer))
  (Variables|Default|SetRewardActor (Class|LearningAgentsManagerListener|GetAgent AgentId "/Game/CharacterAssets/Players/AI/BP_AI_Blue.BP_AI_Blue_C"))
  (bind _hitred (Default|AIShoot (Variables|Default|GetRewardActor)))
  (Variables|/Game/CharacterAssets/Players/AI/BP_AI_Parent.BP_AI_Parent_C|SetWasRanked (Variables|Default|GetRewardActor) false)
  (return (+ (Class|LearningAgentsRewards|MakeRewardonCondition _hitred 1e+01 "ConditionReward" false 0) (Class|LearningAgentsRewards|MakeRewardonCondition (Variables|/Game/CharacterAssets/Players/Player_Parent.Player_Parent_C|GetIsDead (Variables|Default|GetRewardActor)) -0.001 "ConditionReward" false 0) (Class|LearningAgentsRewards|MakeRewardonCondition (Variables|/Game/CharacterAssets/Players/AI/BP_AI_Parent.BP_AI_Parent_C|GetWasRanked (Variables|Default|GetRewardActor)) (Variables|/Game/CharacterAssets/Players/AI/BP_AI_Parent.BP_AI_Parent_C|GetRewardScale (Variables|Default|GetRewardActor)) "ConditionReward" false 0))))

(fn GatherAgentCompletion
  (params (AgentId :type Integer))
  (bind _returnvalue (Class|LearningAgentsManagerListener|GetAgent AgentId "/Game/CharacterAssets/Players/AI/BP_AI_Blue.BP_AI_Blue_C"))
  (if (Variables|/Game/CharacterAssets/Players/AI/BP_AI_Parent.BP_AI_Parent_C|GetShould%20Terminate%20this%20agent _returnvalue)
    (bind _returnvalue_2 (Class|LearningAgentsCompletions|MakeCompletion "Termination" "Completion" false 0))
    (Variables|/Game/CharacterAssets/Players/AI/BP_AI_Parent.BP_AI_Parent_C|SetShould%20Terminate%20this%20agent _returnvalue false))
  (return _returnvalue_2))

(fn ResetAgentEpisode
  (params (AgentId :type Integer))
  (bind _returnvalue (Class|LearningAgentsManagerListener|GetAgent AgentId "/Game/CharacterAssets/Players/AI/BP_AI_Blue.BP_AI_Blue_C"))
  (CallFunction|UselessAgentDetection _returnvalue)
  (Variables|/Game/CharacterAssets/Players/AI/BP_AI_Parent.BP_AI_Parent_C|SetIterationNumber _returnvalue (+ (Variables|/Game/CharacterAssets/Players/AI/BP_AI_Parent.BP_AI_Parent_C|GetIterationNumber _returnvalue) 1))
  (Default|ResettoRandomPoint _returnvalue))

(fn UselessAgentDetection
  (params (ThisAgent :type BP%20AI%20Parent%20Object%20Reference))
  (bind _iterationnumber (Variables|/Game/CharacterAssets/Players/AI/BP_AI_Parent.BP_AI_Parent_C|GetIterationNumber ThisAgent))
  (if (Math|Conversions|ToBoolean(Integer) (Class|KismetMathLibrary|AndIntInt (Math|Conversions|ToInteger(Boolean) (== (Math|Integer|%(Integer) _iterationnumber 5) 0)) (Math|Conversions|ToInteger(Boolean) (!= _iterationnumber 0))))
    (if (== (Variables|/Game/CharacterAssets/Players/AI/BP_AI_Parent.BP_AI_Parent_C|GetHits%20Amount%20By%205%20iterations ThisAgent) 0)
      (Variables|/Game/CharacterAssets/Players/AI/BP_AI_Parent.BP_AI_Parent_C|SetShould%20Terminate%20this%20agent ThisAgent true))
    (Variables|/Game/CharacterAssets/Players/AI/BP_AI_Parent.BP_AI_Parent_C|SetHits%20Amount%20By%205%20iterations ThisAgent 0)))

(fn SetWasCalculatedto0
  (Variables|Default|SetWas%20calculated false))