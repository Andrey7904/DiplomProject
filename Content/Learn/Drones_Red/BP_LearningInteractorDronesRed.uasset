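; Learning Agents interactor for the red AI drone, defining what the agent observes and how it acts.
; Observations hold the drone's location and forward vector plus its NearestEnemy location, all relative to the drone's own transform, so the self readings stay effectively constant.
; Actions are three float axes, written to the drone's XValue, YValue and ZValue variables.
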(fn SpecifyAgentObservation
  (params (InObservationSchema :type Learning%20Agents%20Observation%20Schema%20Object%20Reference))
  (return (Class|LearningAgentsObservations|SpecifyStructObservation InObservationSchema (Utilities|Map|MakeMap "Character" (Class|LearningAgentsObservations|SpecifyStructObservation InObservationSchema (Utilities|Map|MakeMap "Location" (Class|LearningAgentsObservations|SpecifyLocationObservation InObservationSchema 1e+02) "Direction" (Class|LearningAgentsObservations|SpecifyDirectionObservation InObservationSchema))) "Enemy" (Class|LearningAgentsObservations|SpecifyLocationObservation InObservationSchema 1e+02)))))

(fn GatherAgentObservation
  (params (InObservationObject :type Learning%20Agents%20Observation%20Object%20Object%20Reference) (AgentId :type Integer))
  (Variables|Default|SetObsActor (Class|LearningAgentsManagerListener|GetAgent AgentId "/Game/CharacterAssets/Players/AI/Drone/BP_AI_Drone_RED_Final.BP_AI_Drone_RED_Final_C"))
  (return (Class|LearningAgentsObservations|MakeStructObservation InObservationObject (Utilities|Map|MakeMap "Character" (Class|LearningAgentsObservations|MakeStructObservation InObservationObject (Utilities|Map|MakeMap "Location" (Class|LearningAgentsObservations|MakeLocationObservation InObservationObject (Transformation|GetActorLocation (Variables|Default|GetObsActor)) (Transformation|GetActorTransform (Variables|Default|GetObsActor)) "LocationObservation" false 0) "Direction" (Class|LearningAgentsObservations|MakeDirectionObservation InObservationObject (Transformation|GetActorForwardVector (Variables|Default|GetObsActor)) (Transformation|GetActorTransform (Variables|Default|GetObsActor)) "DirectionObservation" false 0))) "Enemy" (Class|LearningAgentsObservations|MakeLocationObservation InObservationObject (Transformation|GetActorLocation (Variables|/Game/CharacterAssets/Players/AI/Drone/BP_AI_Drone_RED_Final.BP_AI_Drone_RED_Final_C|GetNearestEnemy (Variables|Default|GetObsActor))) (Transformation|GetActorTransform (Variables|Default|GetObsActor)) "LocationObservation" false 0)))))

(fn SpecifyAgentAction
  (params (InActionSchema :type Learning%20Agents%20Action%20Schema%20Object%20Reference))
  (return (Class|LearningAgentsActions|SpecifyStructAction InActionSchema (Utilities|Map|MakeMap "Xinput" (Class|LearningAgentsActions|SpecifyFloatAction InActionSchema 1.0) "Yinput" (Class|LearningAgentsActions|SpecifyFloatAction InActionSchema 1.0) "Zinput" (Class|LearningAgentsActions|SpecifyFloatAction InActionSchema 1.0)))))

(fn PerformAgentAction
  (params (InActionObject :type Learning%20Agents%20Action%20Object%20Object%20Reference) (InActionObjectElement :type Learning%20Agents%20Action%20Object%20Element%20Structure%20%28by%20ref%29) (AgentId :type Integer))
  (Variables|Default|SetActActor (Class|LearningAgentsManagerListener|GetAgent AgentId "/Game/CharacterAssets/Players/AI/Drone/BP_AI_Drone_RED_Final.BP_AI_Drone_RED_Final_C"))
  (Class|LearningAgentsActions|GetStructAction InActionObject InActionObjectElement)
  (Utilities|FlowControl|Sequence
    (:then_1
      (bind _outelements (Class|LearningAgentsActions|GetStructAction InActionObject InActionObjectElement))
      (Utilities|FlowControl|Sequence
        (:then_0
          (bind _outvalue (Class|LearningAgentsActions|GetFloatAction InActionObject (.Value (Utilities|Map|Find _outelements "Xinput")) "FloatAction" false 0))
          (Variables|/Game/CharacterAssets/Players/AI/Drone/BP_AI_Drone_RED_Final.BP_AI_Drone_RED_Final_C|SetX_Value (Variables|Default|GetActActor) _outvalue))
        (:then_1
          (bind _outvalue_2 (Class|LearningAgentsActions|GetFloatAction InActionObject (.Value (Utilities|Map|Find _outelements "Yinput")) "FloatAction" false 0))
          (Variables|/Game/CharacterAssets/Players/AI/Drone/BP_AI_Drone_RED_Final.BP_AI_Drone_RED_Final_C|SetY_Value (Variables|Default|GetActActor) _outvalue_2))
        (:then_2
          (bind _outvalue_3 (Class|LearningAgentsActions|GetFloatAction InActionObject (.Value (Utilities|Map|Find _outelements "Zinput")) "FloatAction" false 0))
          (Variables|/Game/CharacterAssets/Players/AI/Drone/BP_AI_Drone_RED_Final.BP_AI_Drone_RED_Final_C|SetZ_Value (Variables|Default|GetActActor) _outvalue_3))))))