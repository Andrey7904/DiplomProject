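; Learning Agents trainer for red AI drones, supplying rewards, completions and episode resets.
; Until an agent's DeadWasCounted flag is set, reward combines hits and a death penalty; the rank bonus never applies because WasRanked is cleared first.
; Completion terminates agents flagged ShouldTerminateThisAgent, and reset moves them to a random point.
; The five-iteration no-hit culling check is disabled, and reward casts to a different drone class than the other functions.
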(fn GatherAgentReward
  (params (AgentId :type Integer))
  (bind _output_get (Variables|Default|SetRewardActor (Class|LearningAgentsManagerListener|GetAgent AgentId "/Game/CharacterAssets/Players/AI/Drone/BP_AI_Drone_RED_Final.BP_AI_Drone_RED_Final_C")))
  (if (Variables|/Game/CharacterAssets/Players/AI/Drone/BP_AI_Drone_RED_Final.BP_AI_Drone_RED_Final_C|GetDeadWasCounted _output_get)
    _
    (else
      (Variables|/Game/CharacterAssets/Players/AI/Drone/BP_AI_Drone_RED_Final.BP_AI_Drone_RED_Final_C|SetWasRanked (Variables|Default|GetRewardActor) false)
      (bind _output_get_2 (Variables|Default|SetTempReward (+ (Class|LearningAgentsRewards|MakeRewardonCondition (!= (Variables|/Game/CharacterAssets/Players/AI/Drone/BP_AI_Drone_RED_Final.BP_AI_Drone_RED_Final_C|GetHitsAmount (Variables|Default|GetRewardActor)) 0) (Math|Conversions|ToFloat(Integer) (* (Variables|/Game/CharacterAssets/Players/AI/Drone/BP_AI_Drone_RED_Final.BP_AI_Drone_RED_Final_C|GetHitsAmount (Variables|Default|GetRewardActor)) 10)) "ConditionReward" false 0) (Class|LearningAgentsRewards|MakeRewardonCondition (Variables|/Game/CharacterAssets/Players/AI/Drone/BP_AI_Drone_RED_Final.BP_AI_Drone_RED_Final_C|GetIsDead (Variables|Default|GetRewardActor)) -1.0 "ConditionReward" false 0) (Class|LearningAgentsRewards|MakeRewardonCondition (Variables|/Game/CharacterAssets/Players/AI/Drone/BP_AI_Drone_RED_Final.BP_AI_Drone_RED_Final_C|GetWasRanked (Variables|Default|GetRewardActor)) (Variables|/Game/CharacterAssets/Players/AI/Drone/BP_AI_Drone_RED_Final.BP_AI_Drone_RED_Final_C|GetReward%20Scale (Variables|Default|GetRewardActor)) "ConditionReward" false 0))))
      (Variables|/Game/CharacterAssets/Players/AI/Drone/BP_AI_Drone_RED_Final.BP_AI_Drone_RED_Final_C|SetHitsAmount (Variables|Default|GetRewardActor) 0)
      (Variables|/Game/CharacterAssets/Players/AI/Drone/BP_AI_Drone_RED_Final.BP_AI_Drone_RED_Final_C|SetDeadWasCounted (Variables|Default|GetRewardActor) true)))
  (return _output_get_2))

(fn GatherAgentCompletion
  (params (AgentId :type Integer))
  (bind _returnvalue (Class|LearningAgentsManagerListener|GetAgent AgentId "/Game/CharacterAssets/Players/AI/AI_Drones/BP_AI_Drone_Red.BP_AI_Drone_Red_C"))
  (if (Variables|/Game/CharacterAssets/Players/BP_Drone.BP_Drone_C|GetShould%20Terminate%20This%20Agent _returnvalue)
    (bind _returnvalue_2 (Class|LearningAgentsCompletions|MakeCompletion "Termination" "Completion" false 0))
    (Variables|/Game/CharacterAssets/Players/BP_Drone.BP_Drone_C|SetShould%20Terminate%20This%20Agent _returnvalue false))
  (return _returnvalue_2))

(fn ResetAgentEpisode
  (params (AgentId :type Integer))
  (bind _returnvalue (Class|LearningAgentsManagerListener|GetAgent AgentId "/Game/CharacterAssets/Players/AI/AI_Drones/BP_AI_Drone_Red.BP_AI_Drone_Red_C"))
  (CallFunction|UselessAgentDetection _returnvalue)
  (Variables|/Game/CharacterAssets/Players/BP_Drone.BP_Drone_C|SetIteration%20Number _returnvalue (+ (Variables|/Game/CharacterAssets/Players/BP_Drone.BP_Drone_C|GetIteration%20Number _returnvalue) 1))
  (Default|ResettoRandomPoint _returnvalue))

(fn UselessAgentDetection
  (params (ThisAgent :type BP%20AI%20Parent%20Object%20Reference))
  (bind _iterationnumber (Variables|/Game/CharacterAssets/Players/AI/BP_AI_Parent.BP_AI_Parent_C|GetIterationNumber ThisAgent))
  (if (Math|Conversions|ToBoolean(Integer) (Class|KismetMathLibrary|AndIntInt (Math|Conversions|ToInteger(Boolean) (== (Math|Integer|%(Integer) _iterationnumber 5) 0)) (Math|Conversions|ToInteger(Boolean) (!= _iterationnumber 0))))
    (if (== (Variables|/Game/CharacterAssets/Players/AI/BP_AI_Parent.BP_AI_Parent_C|GetHits%20Amount%20By%205%20iterations ThisAgent) 0)
      (Variables|/Game/CharacterAssets/Players/AI/BP_AI_Parent.BP_AI_Parent_C|SetShould%20Terminate%20this%20agent ThisAgent true))
    (Variables|/Game/CharacterAssets/Players/AI/BP_AI_Parent.BP_AI_Parent_C|SetHits%20Amount%20By%205%20iterations ThisAgent 0)))

(fn SetWasCalculatedto0
  (Variables|Default|SetWas%20calculated false))