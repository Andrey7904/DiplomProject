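; Learning Agents manager that trains or runs the neural-network policy for red AI drones.
; BeginPlay gathers drones, makes the manager their tick prerequisite, and builds interactor, policy, critic, environment and shared-memory PPO trainer.
; Tick runs inference or training according to RunInference; inference mode also randomizes starting points.
; A hit-based ranking function sets reward scales on BP_AI_Red actors, not the drone class, but its timer is disabled.
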(event EventBeginPlay
  (bind _shared_memory_settings (Variables|Default|GetShared%20Memory%20Settings))
  (Utilities|FlowControl|Sequence
    (:then_0
      (bind _outactors (Actor|GetAllActorsOfClass "/Game/CharacterAssets/Players/AI/Drone/BP_AI_Drone_RED_Final.BP_AI_Drone_RED_Final_C"))
      (bind _output_get (Variables|Default|SetAIActors _outactors))
      (Actor|Tick|AddTickPrerequisiteActor _output_get self))
    (:then_1
      (bind _returnvalue (Class|LearningAgentsInteractor|MakeInteractor (Variables|Default|GetLearningAgentsManager) "/Game/Learn/Drones_Red/BP_LearningInteractorDronesRed.BP_LearningInteractorDronesRed_C" "InteractorDronesRed"))
      (Variables|Default|SetInteractor _returnvalue))
    (:then_2
      (bind _returnvalue_2 (Class|LearningAgentsPolicy|MakePolicy (Variables|Default|GetLearningAgentsManager) (Variables|Default|GetInteractor) "/Script/LearningAgents.LearningAgentsPolicy" "PolicyDronesRed" "/Game/Learn/Drones_Red/DA_NeuralNetworkEncoderDronesRed.DA_NeuralNetworkEncoderDronesRed" "/Game/Learn/Drones_Red/DA_NeuralNetworkPolicyDronesRed.DA_NeuralNetworkPolicyDronesRed" "/Game/Learn/Drones_Red/DA_NeuralNetworkDecoderDronesRed.DA_NeuralNetworkDecoderDronesRed" true true true (Variables|Default|GetPolicy%20Settings) 1234))
      (Variables|Default|SetPolicy _returnvalue_2))
    (:then_3
      (bind _returnvalue_3 (Class|LearningAgentsCritic|MakeCritic (Variables|Default|GetLearningAgentsManager) (Variables|Default|GetInteractor) (Variables|Default|GetPolicy) "/Script/LearningAgents.LearningAgentsCritic" "CriticDronesRed" "/Game/Learn/Drones_Red/DA_NeuralNetworkCriticDronesRed.DA_NeuralNetworkCriticDronesRed" true (Variables|Default|GetCritic%20Settings) 1234))
      (Variables|Default|SetCritic _returnvalue_3))
    (:then_4
      (bind _returnvalue_4 (Class|LearningAgentsTrainingEnvironment|MakeTrainingEnvironment (Variables|Default|GetLearningAgentsManager) "/Game/Learn/Drones_Red/BP_LearningTrainerDronesRed.BP_LearningTrainerDronesRed_C" "TrainingEnvironmentDronesRed"))
      (Variables|Default|SetTraining%20Env _returnvalue_4))
    (:then_5
      (bind _returnvalue_5 (Class|LearningAgentsCommunicatorLibrary|SpawnSharedMemoryTrainingProcess (Variables|Default|GetTrainer%20Process%20Settings) _shared_memory_settings))
      (bind _returnvalue_6 (Class|LearningAgentsCommunicatorLibrary|MakeSharedMemoryCommunicator _returnvalue_5 _shared_memory_settings))
      (Variables|Default|SetCommunicator _returnvalue_6))
    (:then_6
      (bind _returnvalue_7 (Class|LearningAgentsPPOTrainer|MakePPOTrainer (Variables|Default|GetLearningAgentsManager) (Variables|Default|GetInteractor) (Variables|Default|GetTraining%20Env) (Variables|Default|GetPolicy) (Variables|Default|GetCritic) (Variables|Default|GetCommunicator) "/Script/LearningAgentsTraining.LearningAgentsPPOTrainer" "PPOTrainerDronesRed" (Variables|Default|GetTrainer%20Settings)))
      (Variables|Default|SetPPOTrainer _returnvalue_7))
    (:then_7
      (if (Variables|Default|GetRunInference)
        (Default|ResettoRandomPoint (Variables|Default|GetAIActors))))
    (:then_8
      (Utilities|Time|SetTimerbyFunctionName 0 "Calc agent efficiency" 1.9e+02 true)
      (Development|PrintString "SetTimer Ranking ACTIVATED wait 150sec"))))

(event Collision|EventActorBeginOverlap
  (params (OtherActor :type Actor%20Object%20Reference)))

(event EventTick
  (params (DeltaSeconds :type Float%20%28single-precision%29))
  (if (Variables|Default|GetRunInference)
    (Class|LearningAgentsPolicy|RunInference (Variables|Default|GetPolicy) 0.0)
    (else
      (Class|LearningAgentsPPOTrainer|RunTraining (Variables|Default|GetPPOTrainer) (Variables|Default|GetTrainer%20Training%20Settings) (Variables|Default|GetTraining%20Game%20Settings) true true))))

(fn ConstructionScript)

(fn CalcAgentEfficiency
  (bind _hits_amount_array (Variables|Default|GetHits%20Amount%20Array))
  (bind (_indexofminvalue _minvalue) (Math|Float|MinOfFloatArray _hits_amount_array))
  (Development|PrintString "RANKING IN PROGRESS")
  (Utilities|Array|Clear (Variables|Default|GetHits%20Amount%20Array))
  (bind _outactors (Actor|GetAllActorsOfClass "/Game/CharacterAssets/Players/AI/BP_AI_Red.BP_AI_Red_C"))
  (for _array_element _outactors
    (Utilities|Array|Add (Variables|Default|GetHits%20Amount%20Array) (Variables|/Game/CharacterAssets/Players/AI/BP_AI_Parent.BP_AI_Parent_C|GetAmountOfHits _array_element))
    (Variables|Default|SethitsSum (+ (Variables|Default|GethitsSum) (Variables|/Game/CharacterAssets/Players/AI/BP_AI_Parent.BP_AI_Parent_C|GetAmountOfHits _array_element)))
    (Variables|/Game/CharacterAssets/Players/AI/BP_AI_Parent.BP_AI_Parent_C|SetRewardScale _array_element 0.0))
  (Variables|Default|SetAvgHitsAmount (/ (Variables|Default|GethitsSum) (Utilities|Array|Length (Variables|Default|GetHits%20Amount%20Array))))
  (Variables|/Game/CharacterAssets/Players/AI/BP_AI_Parent.BP_AI_Parent_C|SetRewardScale (Utilities|Array|Get(acopy) _outactors (.IndexOfMaxValue (Math|Float|MaxOfFloatArray _hits_amount_array))) 5.0)
  (if (< _minvalue (- (Variables|Default|GetAvgHitsAmount) (* (Variables|Default|GetAvgHitsAmount) 0.8)))
    (Variables|/Game/CharacterAssets/Players/AI/BP_AI_Parent.BP_AI_Parent_C|SetRewardScale (Utilities|Array|Get(acopy) _outactors _indexofminvalue) -5.0)
    (else
      (Variables|/Game/CharacterAssets/Players/AI/BP_AI_Parent.BP_AI_Parent_C|SetRewardScale (Utilities|Array|Get(acopy) _outactors _indexofminvalue) -2.0)))
  (for _array_element_2 _outactors
    (if (< (Variables|/Game/CharacterAssets/Players/AI/BP_AI_Parent.BP_AI_Parent_C|GetAmountOfHits _array_element_2) (- (Variables|Default|GetAvgHitsAmount) (* (Variables|Default|GetAvgHitsAmount) 0.2)))
      (Variables|/Game/CharacterAssets/Players/AI/BP_AI_Parent.BP_AI_Parent_C|SetRewardScale _array_element_2 -1.0)
      (Variables|/Game/CharacterAssets/Players/AI/BP_AI_Parent.BP_AI_Parent_C|SetAmountOfHits _array_element_2 0.0 :!label _label)
      (Variables|/Game/CharacterAssets/Players/AI/BP_AI_Parent.BP_AI_Parent_C|SetWasRanked _array_element_2 true)
      (elif (> (Variables|/Game/CharacterAssets/Players/AI/BP_AI_Parent.BP_AI_Parent_C|GetAmountOfHits _array_element_2) (+ (Variables|Default|GetAvgHitsAmount) (* (Variables|Default|GetAvgHitsAmount) 0.2)))
        (Variables|/Game/CharacterAssets/Players/AI/BP_AI_Parent.BP_AI_Parent_C|SetRewardScale _array_element_2 2.0)
        (goto _label))))
  (return))